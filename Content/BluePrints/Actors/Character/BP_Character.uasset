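; Player character Blueprint with Enhanced Input movement, look and jump, weapon pickup, and melee combo attacks.
; A Peace/Battle/Dead state gates movement and attacks, with repeated attacks queuing the next montage section in NextCombo.
; Collected weapons attach to a hand socket and receive forwarded hit-check begin/end events.
; A DamageReceiver component drives the HP bar and death, while damage also plays a timeline-driven material hit flash.
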(event Custom|Attack
  ;[0.15 0.15 0.15 0.5] 무기 있을때만 공격.
  (if (Variables|Default|GetHasWeapon)
    (switch Utilities|FlowControl|Switch|SwitchonECharacterState (Variables|Default|GetState_BP)
      (:NewEnumerator0
        (Variables|Default|SetState_BP "NewEnumerator1")
        (Animation|PlayAnimMontage "/Game/BluePrints/Actors/Character/AM_CharacterAttack.AM_CharacterAttack" 1.0 "Attack1")
        (Variables|Default|SetIsCanMove false))
      (:NewEnumerator1
        (switch name (Animation|Montage|MontageGetCurrentSection (Components|SkeletalMesh|GetAnimInstance (Variables|Character|GetMesh)) "/Game/BluePrints/Actors/Character/AM_CharacterAttack.AM_CharacterAttack")
          (:Attack1
            (Variables|Default|SetNextCombo "Attack2"))
          (:Attack2
            (Variables|Default|SetNextCombo "Attack3"))
          (:Attack3
            (Variables|Default|SetNextCombo "Attack4"))
          (:Attack4
            (Variables|Default|SetIsCanMove true)))))))

(event Custom|AttackEnd
  (Variables|Default|SetState_BP "NewEnumerator0")
  (Variables|Default|SetNextCombo ""))

(event Custom|OnWeaponCollected
  (params (WeaponActor :type Actor%20Object%20Reference))
  ;[0.15 0.15 0.15 0.5] 무기 수집
  (Actor|SetOwner WeaponActor self)
  (Transformation|AttachComponentToComponent WeaponActor (Variables|Character|GetMesh) "WeaponPosition" "SnapToTarget" "SnapToTarget" "SnapToTarget" true)
  (Variables|Default|SetHasWeapon true)
  (bind _asbp_weapon (Utilities|Casting|CastToBP_Weapon WeaponActor))
  (Variables|Default|Setweapon _asbp_weapon))

(event Custom|OnAttackCheckEnd
  ;[0.15 0.15 0.15 0.5] 무기 수집
  (Default|OnAttackCheckEnd (Variables|Default|Getweapon)))

(event Custom|OnAttackCheckBegin
  ;[0.15 0.15 0.15 0.5] 무기 수집
  (Default|OnAttackCheckBegin (Variables|Default|Getweapon)))

(event Custom|OnDead
  (Collision|SetCollisionEnabled (Variables|Collision|GetCapsuleComponent) "NoCollision")
  (CallFunction|SetState "NewEnumerator2")
  (Variables|/Script/Engine.CharacterMovementComponent|SetMaxWalkSpeed (Variables|Character|GetCharacterMovement) 0.0))

(event Custom|Attacking
  (params (NewParam :type Name))
  (Variables|Default|SetHasUsingWeapon true)
  (Variables|Default|SetNextCombo NewParam)
  (Variables|Default|SetIsCanMove false)
  (Utilities|FlowControl|Delay 0.1)
  (Variables|Default|SetHasUsingWeapon false))

(event Custom|OnHpChanged
  (params (HealthPower :type Float%20%28double-precision%29) (MaxHealthPower :type Float%20%28double-precision%29))
  (Default|SetHPPercent (Variables|Default|GetHPBarObject) (/ HealthPower MaxHealthPower)))

(event Custom|SetState
  (params (NewState :type ECharacterState%20Enum :default "NewEnumerator0"))
  (if (Utilities|Enum|NotEqual(Enum) (Variables|Default|GetState_BP) "NewEnumerator2")
    (if (Utilities|Enum|NotEqual(Enum) NewState (Variables|Default|GetState_BP))
      (Variables|Default|SetState_BP NewState))))

(event Input|EnhancedActionEvents|EnhancedInputActionIA_Move
  (params (ActionValue :type Vector%202D%20Structure) (ElapsedSeconds :type Float%20%28double-precision%29) (TriggeredSeconds :type Float%20%28double-precision%29) (InputAction :type Input%20Action%20Object%20Reference :default "/Game/BluePrints/Actors/Inputs/Actions/IA_Move.IA_Move"))
  ;[0.15 0.15 0.15 0.5] 키보드 입력을 받아 컨트롤러 입력에 사용하기.
  (switch Utilities|FlowControl|Switch|SwitchonECharacterState (Variables|Default|GetState_BP)
    (:NewEnumerator0
      (if (Variables|Default|GetIsCanMove)
        (Pawn|Input|AddMovementInput (* (.y ActionValue) (Math|Vector|GetForwardVector (Math|Rotator|MakeRotator 0.0 0.0 (.yaw (Pawn|GetControlRotation :!class /Script/Engine.Pawn))))) 1.0 false)
        (Pawn|Input|AddMovementInput (* (.x ActionValue) (Math|Vector|GetRightVector (Pawn|GetControlRotation :!class /Script/Engine.Pawn))) 1.0 false)))))

(event Input|EnhancedActionEvents|EnhancedInputActionIA_Attack
  (params (ActionValue :type Boolean) (ElapsedSeconds :type Float%20%28double-precision%29) (TriggeredSeconds :type Float%20%28double-precision%29) (InputAction :type Input%20Action%20Object%20Reference :default "/Game/BluePrints/Actors/Inputs/Actions/IA_Attack.IA_Attack"))
  (CallFunction|Attack))

(event Input|EnhancedActionEvents|EnhancedInputActionIA_Look
  (params (ActionValue :type Vector%202D%20Structure) (ElapsedSeconds :type Float%20%28double-precision%29) (TriggeredSeconds :type Float%20%28double-precision%29) (InputAction :type Input%20Action%20Object%20Reference :default "/Game/BluePrints/Actors/Inputs/Actions/IA_Look.IA_Look"))
  ;[0.15 0.15 0.15 0.5] 마우스 입력을 컨트롤러 회전에 사용하기.
  (Pawn|Input|AddControllerYawInput (.x ActionValue))
  (Pawn|Input|AddControllerPitchInput (.y ActionValue)))

(event Input|EnhancedActionEvents|EnhancedInputActionIA_Jump
  (params (ActionValue :type Boolean) (ElapsedSeconds :type Float%20%28double-precision%29) (TriggeredSeconds :type Float%20%28double-precision%29) (InputAction :type Input%20Action%20Object%20Reference :default "/Game/BluePrints/Actors/Inputs/Actions/IA_Jump.IA_Jump"))
  (Character|Jump))

(event EventBeginPlay
  (bind _damagereceiver (Variables|Default|GetDamageReceiver))
  (bind _returnvalue (Rendering|Material|CreateDynamicMaterialInstance (Variables|Character|GetMesh) 0 "/Game/InfinityBladeWarriors/Characters/TM/CharM_Golden/M_Char_Golden.M_Char_Golden" "None" :!class /Script/Engine.PrimitiveComponent))
  (Variables|Default|SetdynamicInstance _returnvalue)
  (Input|AddMappingContext (PlayerController|LocalPlayerSubsystems|GetEnhancedInputLocalPlayerSubsystem (Game|GetPlayerController 0)) "/Game/BluePrints/Actors/Inputs/IMC_Character.IMC_Character" 0 "(bIgnoreAllPressedKeysUntilRelease=True,bForceImmediately=False,bNotifyUserSettings=False)")
  (bind _aswbp_hp (Utilities|Casting|CastToWBP_HP (UserInterface|GetUserWidgetObject (Variables|Default|GetHPBar))))
  (Variables|Default|SetHPBarObject _aswbp_hp)
  (EventDispatchers|BindEventtoOnDead _damagereceiver (delegate Custom|OnDead))
  (EventDispatchers|AssignOnHealthPowerChanged _damagereceiver (delegate Custom|OnHpChanged)))

(event Game|Damage|EventAnyDamage
  (params (Damage :type Float%20%28single-precision%29) (DamageType :type Damage%20Type%20Object%20Reference) (InstigatedBy :type Controller%20Object%20Reference) (DamageCauser :type Actor%20Object%20Reference))
  (bind _dynamicinstance (Variables|Default|GetdynamicInstance))
  (Default|OnDamageReceived (Variables|Default|GetDamageReceiver) Damage)
  (bind (_direction _value _hitcolor) (Timeline|DamageEffect PlayFromStart)
    (:Update
      (Rendering|Material|SetScalarParameterValue _dynamicinstance "HitValue" _value :!class /Script/Engine.MaterialInstanceDynamic)
      (Rendering|Material|SetVectorParameterValue _dynamicinstance "HitColor" _hitcolor :!class /Script/Engine.MaterialInstanceDynamic))))

(fn ConstructionScript)