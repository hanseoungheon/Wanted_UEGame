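; BP_MyMoving_Platform is a moving platform actor that slides sideways from its starting position.
; On BeginPlay it caches its location and plays a timeline from the start.
; Each timeline update offsets the actor along the right vector of the SMIsCoilsionToyCow component, scaled by the Alpha track and MoveLength.
; Movement sets the location directly without sweeping, so it ignores blocking collisions along the path.
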(event EventBeginPlay
  (Variables|Default|SetOriginalLocation (Transformation|GetActorLocation))
  (bind _alpha (Timeline|Timeline PlayFromStart)
    (:Update
      (Transformation|SetActorLocation (+ (Variables|Default|GetOriginalLocation) (* (Math|Vector|GetRightVector (Variables|Default|GetSM_Is_Coilsion_ToyCow)) (* _alpha (Variables|Default|GetMoveLength)))) false false))))

(event Collision|EventActorBeginOverlap
  (params (OtherActor :type Actor%20Object%20Reference)))

(event EventTick
  (params (DeltaSeconds :type Float%20%28single-precision%29)))

(fn ConstructionScript)