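; BP_DamageReceiver is a component that tracks an actor's health and handles incoming damage.
; Health starts at its maximum on BeginPlay, and damage is subtracted only while the receiver is vulnerable.
; Each accepted hit starts a timed invulnerability window, restored by a timer event.
; Health clamps at zero, and event dispatchers report health changes and death.
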(event Custom|OnDamageReceived
  (params (damage :type Float%20%28double-precision%29))
  ;[0.15 0.15 0.15 0.5] 데미지 처리 공식
  (if (Variables|Default|GetVulnerable)
    (Variables|Default|SetVulnerable false)
    (Utilities|Time|SetTimerbyEvent (delegate Custom|ReturnToVulnerable) (Variables|Default|GetInVulerableTime))
    (Variables|Default|SetHealthPower (- (Variables|Default|GetHealthPower) damage))
    (if (<= (Variables|Default|GetHealthPower) 0.0)
      (Variables|Default|SetHealthPower 0.0)
      (Default|CallOnDead)
      (Default|CallOnHealthPowerChanged (Variables|Default|GetHealthPower) (Variables|Default|GetMaxHealthPower))
      (else
        (Default|CallOnHealthPowerChanged (Variables|Default|GetHealthPower) (Variables|Default|GetMaxHealthPower))))))

(event Custom|ReturnToVulnerable
  ;[0.15 0.15 0.15 0.5] 데미지 처리 공식
  (Variables|Default|SetVulnerable true))

(event EventBeginPlay
  (Variables|Default|SetHealthPower (Variables|Default|GetMaxHealthPower)))