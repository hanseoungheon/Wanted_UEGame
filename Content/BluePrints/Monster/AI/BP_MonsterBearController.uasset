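; AI controller for the bear monster that starts its behavior when it possesses a pawn.
; On possess it applies the BB_MonsterBear blackboard and seeds it with the patrol wait time and the pawn's current location as its original location.
; It then runs the BT_MonsterBear behavior tree, which takes over the bear's decisions.
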(event EventBeginPlay)

(event EventTick
  (params (DeltaSeconds :type Float%20%28single-precision%29)))

(event EventPossess
  (params (PossessedPawn :type Pawn%20Object%20Reference))
  (Utilities|FlowControl|Sequence
    (:then_0
      (Class|AIController|UseBlackboard "/Game/BluePrints/Monster/AI/BB_MonsterBear.BB_MonsterBear")
      (AI|Components|Blackboard|SetValueasFloat (Variables|Default|GetBlackboard) (Variables|Default|GetPatrol%20Wait%20Time%20Key) (Variables|Default|GetPatrol%20Wait%20Time))
      (AI|Components|Blackboard|SetValueasVector (Variables|Default|GetBlackboard) (Variables|Default|GetOriginal%20Location%20Key) (Transformation|GetActorLocation PossessedPawn)))
    (:then_1
      (AI|RunBehaviorTree "/Game/BluePrints/Monster/AI/BT_MonsterBear.BT_MonsterBear"))))

(fn ConstructionScript)