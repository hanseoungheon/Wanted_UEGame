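; Bear enemy that chases and attacks the player, with stats from MonsterData and an HP bar widget.
; SetState mirrors Peace/Chase/Attack/Dead to the AI blackboard and sets speed; PawnSensing starts chases, Tick checks when to disengage.
; Attack events toggle a hitbox that applies damage on overlap.
; DamageReceiver events update HP, trigger brief flinches and handle death, with timelines driving material hit flash and dissolve before destruction.
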(event OnSeePawn(PawnSensing)
  (params (Pawn :type Pawn%20Object%20Reference))
  (switch Utilities|FlowControl|Switch|SwitchonEMonsterState (Variables|Default|GetState_BP)
    (:NewEnumerator0
      (bind _asbp_character (Utilities|Casting|CastToBP_Character Pawn))
      (if (Utilities|Enum|NotEqual(Enum) (Variables|/Game/BluePrints/Actors/Character/BP_Character.BP_Character_C|GetState_BP _asbp_character) "NewEnumerator2")
        (AI|Components|Blackboard|SetValueasObject (Variables|/Script/AIModule.AIController|GetBlackboard (AI|GetAIController self)) (Variables|Default|GetTargetPlayerKey) Pawn)
        (CallFunction|SetState "NewEnumerator1")))))

(event OnComponentBeginOverlap(AttackCollision)
  (params (OverlappedComponent :type Primitive%20Component%20Object%20Reference) (OtherActor :type Actor%20Object%20Reference) (OtherComp :type Primitive%20Component%20Object%20Reference) (OtherBodyIndex :type Integer) (bFromSweep :type Boolean) (SweepResult :type Hit%20Result%20Structure%20%28by%20ref%29))
  (Game|Damage|ApplyDamage OtherActor (.attack (Default|GetCurrentDataLevel (Variables|Default|GetMonsterData))) (AI|GetAIController self) self))

(event Custom|RotateHPBar
  (params (HPBatR :type Rotator))
  (Transformation|SetRelativeRotation (Variables|Default|GetHPBar) HPBatR false false))

(event Custom|OnMonster%20Dead
  (bind _dynamicinstance (Variables|Default|GetdynamicInstance))
  ;[0.15 0.15 0.15 0.5] 죽으면 콜리전 끄기
  (Collision|SetCollisionEnabled (Variables|Collision|GetCapsuleComponent) "NoCollision")
  (Collision|SetCollisionEnabled (Variables|Default|GetAttack%20Collision) "NoCollision")
  (CallFunction|SetState "NewEnumerator3")
  (Rendering|Material|SetScalarParameterValue (Variables|Default|GetdynamicInstance) "Eye Glow Intensity" 0.0 :!class /Script/Engine.MaterialInstanceDynamic)
  (Development|PrintString "몬스터 사망" true true "(R=1.000000,G=0.161129,B=0.255890,A=1.000000)" 1e+01)
  (Utilities|FlowControl|Delay 2.0)
  (bind _dissolve (Timeline|Disslove PlayFromStart)
    (:Update
      (Rendering|Material|SetScalarParameterValue _dynamicinstance "Disslove" _dissolve :!class /Script/Engine.MaterialInstanceDynamic)
      (Rendering|Material|SetScalarParameterValue _dynamicinstance "HitValue" (* _dissolve 1e+02) :!class /Script/Engine.MaterialInstanceDynamic))
    (:Finished
      (Actor|DestroyActor))))

(event Custom|SetState
  (params (NewState :type EMonsterState%20Enum :default "NewEnumerator0"))
  (bind _monsterdata (Variables|Default|GetMonsterData))
  (bind _currentleveldata (Default|GetCurrentDataLevel _monsterdata))
  (if (Utilities|Enum|NotEqual(Enum) (Variables|Default|GetState_BP) "NewEnumerator3")
    (if (Utilities|Enum|NotEqual(Enum) NewState (Variables|Default|GetState_BP))
      (AI|Components|Blackboard|SetValueasEnum (AI|GetBlackboard (AI|GetAIController self)) (Variables|Default|GetStateKey) NewState)
      (bind _output_get (Variables|Default|SetState_BP NewState))
      (switch Utilities|FlowControl|Switch|SwitchonEMonsterState _output_get
        (:NewEnumerator0
          (Variables|/Script/Engine.CharacterMovementComponent|SetMaxWalkSpeed (Variables|Character|GetCharacterMovement) (.walkspeed _currentleveldata))
          (AI|Components|Blackboard|SetValueasObject (AI|GetBlackboard (AI|GetAIController self)) (Variables|Default|GetTargetPlayerKey) 0))
        (:NewEnumerator1
          (Variables|/Script/Engine.CharacterMovementComponent|SetMaxWalkSpeed (Variables|Character|GetCharacterMovement) (.chasespeed _currentleveldata)))
        (:NewEnumerator2
          (Variables|/Script/Engine.CharacterMovementComponent|SetMaxWalkSpeed (Variables|Character|GetCharacterMovement) 0.0 :!label _label))
        (:NewEnumerator3
          (goto _label))))))

(event Custom|움찔
  (params (HealthPower :type Float%20%28double-precision%29) (MaxHealthPower :type Float%20%28double-precision%29))
  (if (not (Variables|Default|GetIsHit))
    (if (> (Variables|/Game/BluePrints/Components/BP_DamageReceiver.BP_DamageReceiver_C|GetHealthPower (Variables|Default|GetDamageReceiver)) 0.0)
      (if (Utilities|Enum|NotEqual(Enum) (Variables|Default|GetState_BP) "NewEnumerator3")
        (Variables|Default|SetIsHit true)
        (Variables|Default|SetState_BP "NewEnumerator4")
        (Utilities|FlowControl|Delay 0.1)
        (Variables|Default|SetState_BP "NewEnumerator0")
        (Variables|Default|SetIsHit false)))))

(event Custom|OnHpChanged
  (params (HealthPower :type Float%20%28double-precision%29) (MaxHealthPower :type Float%20%28double-precision%29))
  (Default|SetHPPercent (Variables|Default|GetHPBarObject) (/ HealthPower MaxHealthPower))
  (CallFunction|움찔 0.0 0.0))

(event Custom|OnAttackCheckBegin
  (Collision|SetCollisionEnabled (Variables|Default|GetAttack%20Collision) "QueryOnly"))

(event Custom|OnAttackCheckEnd
  (Collision|SetCollisionEnabled (Variables|Default|GetAttack%20Collision) "NoCollision"))

(event Custom|TurnToTarget
  (params (TargetActor :type Actor%20Object%20Reference))
  (Transformation|SetActorRotation (Math|Rotator|MakeRotfromX (- (Transformation|GetActorLocation TargetActor) (Transformation|GetActorLocation)))))

(event EventBeginPlay
  (bind _returnvalue (Rendering|Material|CreateDynamicMaterialInstance (Variables|Character|GetMesh) 0 "/Game/InfinityBladeAdversaries/Enemy/Enemy_Bear/Materials/M_Bear_Polar_Inst.M_Bear_Polar_Inst" "None" :!class /Script/Engine.PrimitiveComponent))
  (Variables|Default|SetdynamicInstance _returnvalue)
  ;[0.15 0.15 0.15 0.5] OnDead이벤트 함수 구독
  (EventDispatchers|BindEventtoOnDead (Variables|Default|GetDamageReceiver) (delegate Custom|OnMonster%20Dead))
  (bind _aswbp_hp (Utilities|Casting|CastToWBP_HP (UserInterface|GetUserWidgetObject (Variables|Default|GetHPBar))))
  (Variables|Default|SetHPBarObject _aswbp_hp)
  (EventDispatchers|BindEventtoOnHealthPowerChanged (Variables|Default|GetDamageReceiver) (delegate Custom|OnHpChanged))
  (Variables|/Script/Engine.CharacterMovementComponent|SetMaxWalkSpeed (Variables|Character|GetCharacterMovement) (.walkspeed (Default|GetCurrentDataLevel (Variables|Default|GetMonsterData)))))

(event Collision|EventActorBeginOverlap
  (params (OtherActor :type Actor%20Object%20Reference)))

(event EventTick
  (params (DeltaSeconds :type Float%20%28single-precision%29))
  (switch Utilities|FlowControl|Switch|SwitchonEMonsterState (Variables|Default|GetState_BP)
    (:NewEnumerator1
      (CallFunction|OnChase))
    (:NewEnumerator2
      (CallFunction|OnAttack))))

(event Game|Damage|EventAnyDamage
  (params (Damage :type Float%20%28single-precision%29) (DamageType :type Damage%20Type%20Object%20Reference) (InstigatedBy :type Controller%20Object%20Reference) (DamageCauser :type Actor%20Object%20Reference))
  (bind _dynamicinstance (Variables|Default|GetdynamicInstance))
  ;[0.15 0.15 0.15 0.5] 데미지 처리.
  (Default|OnDamageReceived (Variables|Default|GetDamageReceiver) Damage)
  (bind _value (Timeline|HitEffect PlayFromStart)
    (:Update
      (Rendering|Material|SetScalarParameterValue _dynamicinstance "HitValue" _value :!class /Script/Engine.MaterialInstanceDynamic)
      (Rendering|Material|SetVectorParameterValue :self _dynamicinstance :!class /Script/Engine.MaterialInstanceDynamic))))

(fn ConstructionScript)

(fn OnChase
  (bind _asactor (Utilities|Casting|CastToActor (AI|Components|Blackboard|GetValueasObject (AI|GetBlackboard (AI|GetAIController self)) (Variables|Default|GetTargetPlayerKey))))
  (if (> (Transformation|GetDistanceTo _asactor) (Variables|/Script/AIModule.PawnSensingComponent|GetSightRadius (Variables|Default|GetPawnSensing)))
    (CallFunction|SetState "NewEnumerator0")))

(fn OnAttack
  (bind _asbp_character (Utilities|Casting|CastToBP_Character (AI|Components|Blackboard|GetValueasObject (AI|GetBlackboard (AI|GetAIController self)) (Variables|Default|GetTargetPlayerKey))))
  (if (Utilities|Enum|Equal(Enum) (Variables|/Game/BluePrints/Actors/Character/BP_Character.BP_Character_C|GetState_BP _asbp_character) "NewEnumerator2")
    (CallFunction|SetState "NewEnumerator0")))